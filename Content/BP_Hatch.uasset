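; BP_Hatch is a roof hatch that serves as a level exit, opening for a required item and triggering the win screen.
; Its Interaction event checks that the player's first inventory item is named "El_Doss", then plays a one-time Timeline that rotates and moves the hatch.
; A separate box overlap by the third-person character shows Win_Menu with UI-only input and a visible cursor, without checking whether the hatch is open.
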(event `/Game/BPI_Interact.Interaction`
  (params (DirectionInteract :type "Vector Structure") (PlayerRef :type "/Game/ThirdPerson/Blueprints/BP_ThirdPersonCharacter Object Reference"))
  (bind _roof_hatch (`self.Roof_Hatch`))
  (if (== (`.Item_Name_2_634492BF42674EF4DC449DA84C3E2BCD` (break `/Game/InventorySystem/ItemInformation` (`|GetArrayItem` (`/Game/ThirdPerson/Blueprints/BP_ThirdPersonCharacter.ItemsArray` PlayerRef)))) "El_Doss")
    (`/Engine/EditorBlueprintResources/StandardMacros.DoOnce` false
      (:`Completed`
        (bind (_direction _rotation _y _z) (`Timeline|Timeline` :!via `PlayFromStart`)
          (:`Update`
            (`SceneComponent.K2_SetRelativeRotation` _roof_hatch (`KismetMathLibrary.RLerp` (struct) (struct :`Roll` 90.0) _rotation) false false)
            (`SceneComponent.K2_SetRelativeLocation` _roof_hatch (`KismetMathLibrary.MakeVector` 0.0 _y _z) false false)))))))

(event `self.Box.OnComponentBeginOverlap`
  (params (OverlappedComponent :type "PrimitiveComponent Object Reference") (OtherActor :type "Actor Object Reference") (OtherComp :type "PrimitiveComponent Object Reference") (OtherBodyIndex :type Integer) (bFromSweep :type Boolean) (SweepResult :type "HitResult Structure (by ref)"))
  (bind _returnvalue (`GameplayStatics.GetPlayerController` 0))
  (cast `/Game/ThirdPerson/Blueprints/BP_ThirdPersonCharacter` OtherActor)
  (bind _returnvalue_2 (`|CreateWidget` "/Game/UI/BP/Win_Menu.Win_Menu_C"))
  (`UserWidget.AddToViewport` _returnvalue_2 0)
  (`WidgetBlueprintLibrary.SetInputMode_UIOnlyEx` _returnvalue _returnvalue_2)
  (set `PlayerController.bShowMouseCursor` true _returnvalue))

(fn `UserConstructionScript`)