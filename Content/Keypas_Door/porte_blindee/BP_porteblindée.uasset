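; Armored door Blueprint gated by a wire check and a keypad widget.
; Overlap with the third-person character enables input; leaving disables it, removes the Numpad and restores game-only input.
; Interact opens the Numpad in game-and-UI mode only if the referenced wire's Win flag is set.
; A separate OpenTheDoor event plays a Timeline animating the door mesh's relative location and yaw.
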(event `Interact`
  (bind _returnvalue (`GameplayStatics.GetPlayerController` 0))
  (bind _wire_ref (`self.Wire Ref`))
  (`/Engine/EditorBlueprintResources/StandardMacros.IsValid` _wire_ref
    (:`Is Valid`
      (if (`/Game/BP_WirePuzzle.Win` _wire_ref)
        (bind _returnvalue_2 (`|CreateWidget` "/Game/Keypas_Door/Numpad.Numpad_C"))
        (`UserWidget.AddToViewport` _returnvalue_2 0)
        (`WidgetBlueprintLibrary.SetInputMode_GameAndUIEx` _returnvalue null)
        (set `PlayerController.bShowMouseCursor` false _returnvalue)))))

(event `self.porte_blindee.OnComponentBeginOverlap`
  (params (OverlappedComponent :type "PrimitiveComponent Object Reference") (OtherActor :type "Actor Object Reference") (OtherComp :type "PrimitiveComponent Object Reference") (OtherBodyIndex :type Integer) (bFromSweep :type Boolean) (SweepResult :type "HitResult Structure (by ref)"))
  (cast `/Game/ThirdPerson/Blueprints/BP_ThirdPersonCharacter` OtherActor)
  (`self.EnableInput` (`GameplayStatics.GetPlayerController` 0)))

(event `OpenTheDoor`
  (bind (_direction _newtrack_0 _rotation) (`Timeline|Timeline` :!via `PlayFromStart`)
    (:`Update`
      (`SceneComponent.K2_SetRelativeLocationAndRotation` (`self.porte_blindee`) _newtrack_0 (`KismetMathLibrary.MakeRotator` 0.0 0.0 _rotation) false false))))

(event `self.porte_blindee.OnComponentEndOverlap`
  (params (OverlappedComponent :type "PrimitiveComponent Object Reference") (OtherActor :type "Actor Object Reference") (OtherComp :type "PrimitiveComponent Object Reference") (OtherBodyIndex :type Integer))
  (bind _returnvalue (`GameplayStatics.GetPlayerController` 0))
  (cast `/Game/ThirdPerson/Blueprints/BP_ThirdPersonCharacter` OtherActor)
  (`self.DisableInput` (`GameplayStatics.GetPlayerController` 0))
  (`Widget.RemoveFromParent` (stale `Interact` _returnvalue_2))
  (`WidgetBlueprintLibrary.SetInputMode_GameOnly` _returnvalue)
  (set `PlayerController.bShowMouseCursor` false _returnvalue))

(fn `UserConstructionScript`)